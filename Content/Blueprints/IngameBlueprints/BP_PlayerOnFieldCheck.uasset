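; BP_PlayerOnFieldCheck is a trigger volume that tells the day/night manager whether the player is on the field at night.
; When the player character enters the Box during night, it sets PlayerOnField on DayNightManagerRef and calls StartTimer.
; Exiting clears the flag regardless of time of day, without stopping the timer here.
; Night is checked only on entry, so nightfall while the player is already inside triggers nothing here.
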(event OnComponentBeginOverlap(Box)
  (params (OverlappedComponent :type Primitive%20Component%20Object%20Reference) (OtherActor :type Actor%20Object%20Reference) (OtherComp :type Primitive%20Component%20Object%20Reference) (OtherBodyIndex :type Integer) (bFromSweep :type Boolean) (SweepResult :type Hit%20Result%20Structure%20%28by%20ref%29))
  (bind _daynightmanagerref (Variables|Default|GetDayNightManagerRef))
  (if (== OtherActor (Game|GetPlayerCharacter 0))
    (if (Variables|/Game/Blueprints/IngameBlueprints/BP_DayNightManager.BP_DayNightManager_C|GetIsNight? _daynightmanagerref)
      (Variables|/Game/Blueprints/IngameBlueprints/BP_DayNightManager.BP_DayNightManager_C|SetPlayerOnField? _daynightmanagerref true)
      (Default|StartTimer _daynightmanagerref))))

(event OnComponentEndOverlap(Box)
  (params (OverlappedComponent :type Primitive%20Component%20Object%20Reference) (OtherActor :type Actor%20Object%20Reference) (OtherComp :type Primitive%20Component%20Object%20Reference) (OtherBodyIndex :type Integer))
  (if (== OtherActor (Game|GetPlayerCharacter 0))
    (Variables|/Game/Blueprints/IngameBlueprints/BP_DayNightManager.BP_DayNightManager_C|SetPlayerOnField? (Variables|Default|GetDayNightManagerRef) false)))

(fn ConstructionScript)