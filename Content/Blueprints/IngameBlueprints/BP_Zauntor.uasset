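; BP_Zauntor is a two-leaf fence gate that opens at day start and closes when the player crosses a trigger at night.
; It binds to the day-night manager's begin-day dispatcher, while a second trigger hides the night exclamation marker.
; Opening and closing play a sound, snap a Cube up or down, and slide the leaves via separate timelines.
; The timeline named ZaunOpen drives closing.
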(event OnComponentBeginOverlap(Box)
  (params (OverlappedComponent :type Primitive%20Component%20Object%20Reference) (OtherActor :type Actor%20Object%20Reference) (OtherComp :type Primitive%20Component%20Object%20Reference) (OtherBodyIndex :type Integer) (bFromSweep :type Boolean) (SweepResult :type Hit%20Result%20Structure%20%28by%20ref%29))
  (Utilities|Casting|CastToBP_Player OtherActor)
  (if (Variables|/Game/Blueprints/IngameBlueprints/BP_DayNightManager.BP_DayNightManager_C|GetIsNight? (Variables|Default|GetDayNightManagerRef))
    (Rendering|SetActorHiddenInGame (Variables|Default|GetNightAusrufezeichen) true)))

(event OnComponentBeginOverlap(Box1)
  (params (OverlappedComponent :type Primitive%20Component%20Object%20Reference) (OtherActor :type Actor%20Object%20Reference) (OtherComp :type Primitive%20Component%20Object%20Reference) (OtherBodyIndex :type Integer) (bFromSweep :type Boolean) (SweepResult :type Hit%20Result%20Structure%20%28by%20ref%29))
  (Utilities|Casting|CastToBP_Player OtherActor)
  (if (Variables|/Game/Blueprints/IngameBlueprints/BP_DayNightManager.BP_DayNightManager_C|GetIsNight? (Variables|Default|GetDayNightManagerRef))
    (CallFunction|ZauntorZu)))

(event Custom|ZauntorZu
  (Audio|PlaySound2D "/Game/Assets/Sound/SFX/SC_Zauntor.SC_Zauntor" 1.0 1.0 0.0 0 0)
  (Transformation|SetRelativeLocation (Variables|Default|GetCube) "0.000000,-13.000000,153.000000" false false)
  (bind _alpha (Timeline|ZaunOpen Play)
    (:Update
      (Transformation|SetRelativeLocation (Variables|Default|GetZaunTorR) (Math|Vector|Lerp(Vector) "-120.000000,0.000000,0.000000" "0, 0, 0" _alpha) false false)
      (Transformation|SetRelativeLocation (Variables|Default|GetZaunTorL) (Math|Vector|Lerp(Vector) "120.000000,0.000000,0.000000" "0, 0, 0" _alpha) false false))))

(event Custom|ZauntorAuf
  (Audio|PlaySound2D "/Game/Assets/Sound/SFX/SC_Zauntor.SC_Zauntor" 1.0 1.0 0.0 0 0)
  (Transformation|SetRelativeLocation (Variables|Default|GetCube) "0.000000,-13.000000,450.000000" false false)
  (bind _alpha (Timeline|Timeline Play)
    (:Update
      (Transformation|SetRelativeLocation (Variables|Default|GetZaunTorR) (Math|Vector|Lerp(Vector) "0, 0, 0" "-120.000000,0.000000,0.000000" _alpha) false false)
      (Transformation|SetRelativeLocation (Variables|Default|GetZaunTorL) (Math|Vector|Lerp(Vector) "0, 0, 0" "120.000000,0.000000,0.000000" _alpha) false false))))

(event Custom|DayTorauf
  (CallFunction|ZauntorAuf))

(event EventBeginPlay
  (EventDispatchers|BindEventtoBeginDayDispatcher (Variables|Default|GetDayNightManagerRef) (delegate Custom|DayTorauf)))

(fn ConstructionScript)