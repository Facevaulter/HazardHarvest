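; BP_CabbagePlantMutant is a mutant cabbage plant that periodically stomps to stun nearby players.
; A looping timer started at BeginPlay calls TryStomping at StompInterval, which triggers StompAttack behind an IsStomping flag.
; StompAttack clears the flag immediately, then sphere-overlaps StompRange around the plant for BP_Player pawns and calls Stunned on each.
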(event Custom|TryStomping
  (if (not (Variables|Default|GetIsStomping))
    (Variables|Default|SetIsStomping true)
    (CallFunction|StompAttack)))

(event Custom|StompAttack
  (Variables|Default|SetIsStomping false)
  (bind _outactors (Collision|SphereOverlapActors (Transformation|GetActorLocation) (Variables|Default|GetStompRange) (Utilities|Array|MakeArray "ObjectTypeQuery3") "/Game/Blueprints/Core/BP_Player.BP_Player_C"))
  (for _array_element _outactors
    (bind _asbp_player (Utilities|Casting|CastToBP_Player _array_element))
    (Default|Stunned _asbp_player 0.0)))

(event EventBeginPlay
  (Utilities|Time|SetTimerbyEvent (delegate Custom|TryStomping) (Variables|Default|GetStompInterval) true))

(fn ConstructionScript
  (|CallParentFunction))