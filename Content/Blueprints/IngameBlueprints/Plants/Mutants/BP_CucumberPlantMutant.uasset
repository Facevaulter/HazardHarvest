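; BP_CucumberPlantMutant is a cucumber plant mutant enemy that knocks the player back with a spin attack, then stuns them.
; While the player is in AggroRange, a looping timer calls TryAttack, which attacks only if an AttackRange overlap has set CanAttack.
; The attack plays a spin montage and sound, then launches the player away from the plant.
; A polling timer waits until the player is walking again before applying the stun and re-enabling hits.
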(event OnComponentBeginOverlap(AttackRange)
  (params (OverlappedComponent :type Primitive%20Component%20Object%20Reference) (OtherActor :type Actor%20Object%20Reference) (OtherComp :type Primitive%20Component%20Object%20Reference) (OtherBodyIndex :type Integer) (bFromSweep :type Boolean) (SweepResult :type Hit%20Result%20Structure%20%28by%20ref%29))
  (if (== OtherActor (Game|GetPlayerCharacter 0))
    (if (Variables|Default|GetCanHit)
      (Variables|Default|SetCanAttack true))))

(event OnComponentBeginOverlap(AggroRange)
  (params (OverlappedComponent :type Primitive%20Component%20Object%20Reference) (OtherActor :type Actor%20Object%20Reference) (OtherComp :type Primitive%20Component%20Object%20Reference) (OtherBodyIndex :type Integer) (bFromSweep :type Boolean) (SweepResult :type Hit%20Result%20Structure%20%28by%20ref%29))
  (bind _returnvalue (Game|GetPlayerCharacter 0))
  (if (== OtherActor _returnvalue)
    (bind _asbp_player (Utilities|Casting|CastToBP_Player _returnvalue))
    (Variables|Default|SetPlayerRef _asbp_player)
    (Utilities|Time|SetTimerbyFunctionName 0 "TryAttack" 1.0 true)))

(event OnComponentEndOverlap(AttackRange)
  (params (OverlappedComponent :type Primitive%20Component%20Object%20Reference) (OtherActor :type Actor%20Object%20Reference) (OtherComp :type Primitive%20Component%20Object%20Reference) (OtherBodyIndex :type Integer))
  (if (== OtherActor (Game|GetPlayerCharacter 0))
    (Variables|Default|SetCanAttack false)))

(event OnComponentEndOverlap(AggroRange)
  (params (OverlappedComponent :type Primitive%20Component%20Object%20Reference) (OtherActor :type Actor%20Object%20Reference) (OtherComp :type Primitive%20Component%20Object%20Reference) (OtherBodyIndex :type Integer))
  (if (== OtherActor (Game|GetPlayerCharacter 0))
    (Class|KismetSystemLibrary|PauseTimer 0 "TryAttack")))

(event Custom|SuccessfulHit
  (bind _returnvalue (Transformation|GetActorLocation))
  (bind _playerref (Variables|Default|GetPlayerRef))
  (bind _throwbackstrength (Variables|Default|GetThrowbackStrength))
  (bind _returnvalue_2 (Transformation|GetActorLocation _playerref))
  (bind _returnvalue_3 (- _returnvalue_2 _returnvalue))
  (bind _returnvalue_4 (Math|Vector|Normalize _returnvalue_3 1.0))
  (bind _returnvalue_5 (* _returnvalue_4 _throwbackstrength))
  (bind (_x _y) (Math|Vector|BreakVector _returnvalue_5))
  (bind _playerref_2 (Variables|Default|GetPlayerRef)
    (:then
      (Character|LaunchCharacter _playerref_2 (Math|Vector|MakeVector _x _y 3e+02) true false)
      (Variables|Default|SetCanAttack false)
      (Variables|Default|SetCanHit false)
      (Utilities|Time|SetTimerbyFunctionName 0 "GroundedCheck" 0.2 true))
    (:else)))

(event Custom|ResetMovement
  (Class|KismetSystemLibrary|PauseTimer 0 "GroundedCheck")
  (Variables|Default|SetCanHit true))

(event EventBeginPlay
  (bind _asabp_cucumber (Utilities|Casting|CastToABP_Cucumber (Components|SkeletalMesh|GetAnimInstance (Variables|Default|GetSkeletalMesh))))
  (Variables|Default|SetABPCucumberRef _asabp_cucumber))

(fn ConstructionScript
  (|CallParentFunction))

(fn TryAttack
  (if (Variables|Default|GetCanAttack)
    (Animation|Montage|MontagePlay (Variables|Default|GetABPCucumberRef) "/Game/Assets/Meshes/Plants/Gurke/AM_CucumberSpin.AM_CucumberSpin" 1.0 "MontageLength" 0.0 true)
    (Audio|PlaySound2D "/Game/Assets/Sound/SFX/MutantPlants/Cucumber/SC_CucumberSpin.SC_CucumberSpin" 1.0 1.0 0.0 0 0)
    (CallFunction|SuccessfulHit)))

(fn GroundedCheck
  (bind _playerref (Variables|Default|GetPlayerRef)
    (:then
      (if (Utilities|Enum|Equal(Enum) (Variables|/Script/Engine.CharacterMovementComponent|GetMovementMode (Variables|/Script/Engine.Character|GetCharacterMovement _playerref)) "MOVE_Walking")
        (Default|Stunned _playerref (Variables|Default|GetStun%20Duration))
        (CallFunction|ResetMovement)))
    (:else)))