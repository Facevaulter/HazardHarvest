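; BP_CornProjectile is a projectile from the mutant corn plant that stuns the player on contact.
; Its hitbox overlap calls Stunned on BP_Player with a stun duration, then destroys the projectile.
; It also destroys itself after its lifetime expires or when the BP_DayNightManager begin-day dispatcher fires, unbinding from that dispatcher in the latter case.
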(event OnComponentBeginOverlap(Hitbox)
  (params (OverlappedComponent :type Primitive%20Component%20Object%20Reference) (OtherActor :type Actor%20Object%20Reference) (OtherComp :type Primitive%20Component%20Object%20Reference) (OtherBodyIndex :type Integer) (bFromSweep :type Boolean) (SweepResult :type Hit%20Result%20Structure%20%28by%20ref%29))
  (bind _returnvalue (Game|GetPlayerCharacter 0))
  (if (== OtherActor _returnvalue)
    (bind _asbp_player (Utilities|Casting|CastToBP_Player _returnvalue))
    (Default|Stunned _asbp_player (Variables|Default|GetStun%20Duration))
    (Utilities|IsValid self
      (:Is%20Valid
        (Actor|DestroyActor)))))

(event Custom|DestroyOnDay
  (Utilities|IsValid self
    (:Is%20Valid
      (EventDispatchers|UnbindEventfromBeginDayDispatcher (stale EventBeginPlay _output_get) (delegate Custom|DestroyOnDay))
      (Actor|DestroyActor))))

(event EventBeginPlay
  (bind _returnvalue (Actor|GetActorOfClass "/Game/Blueprints/IngameBlueprints/BP_DayNightManager.BP_DayNightManager_C"))
  (bind _output_get (Variables|Default|SetDayNightManagerRef _returnvalue))
  (EventDispatchers|BindEventtoBeginDayDispatcher _output_get (delegate Custom|DestroyOnDay))
  (Utilities|FlowControl|Delay (Variables|Default|GetLifeTime))
  (Utilities|IsValid self
    (:Is%20Valid
      (Actor|DestroyActor))))

(fn ConstructionScript)