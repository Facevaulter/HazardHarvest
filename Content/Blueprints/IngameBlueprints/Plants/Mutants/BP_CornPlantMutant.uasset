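; Corn plant mutant enemy that turns toward the player and fires projectiles while they are in its aggro range.
; Entering range starts looping timers that yaw the Cylinder at the player, pausing during shots, and play the ABP_Corn shoot montage.
; ShootProjectile, not called here, spawns projectiles with slight random yaw.
; Leaving range clears the player and pauses aiming, but targets ShootProjectile's timer rather than the looping BeginShootAnim one.
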(event OnComponentBeginOverlap(AggroRange)
  (params (OverlappedComponent :type Primitive%20Component%20Object%20Reference) (OtherActor :type Actor%20Object%20Reference) (OtherComp :type Primitive%20Component%20Object%20Reference) (OtherBodyIndex :type Integer) (bFromSweep :type Boolean) (SweepResult :type Hit%20Result%20Structure%20%28by%20ref%29))
  (bind _returnvalue (Game|GetPlayerCharacter 0))
  (if (== OtherActor _returnvalue)
    (bind _asbp_player (Utilities|Casting|CastToBP_Player _returnvalue))
    (Variables|Default|SetPlayerRef _asbp_player)
    (bind _returnvalue_2 (Utilities|Time|SetTimerbyEvent (delegate Custom|LookAtPlayer) 0.01 true))
    (Variables|Default|SetLookEventTimeHandle _returnvalue_2)
    (Utilities|Time|SetTimerbyFunctionName 0 "BeginShootAnim" (Variables|Default|GetAttackInterval) true)))

(event OnComponentEndOverlap(AggroRange)
  (params (OverlappedComponent :type Primitive%20Component%20Object%20Reference) (OtherActor :type Actor%20Object%20Reference) (OtherComp :type Primitive%20Component%20Object%20Reference) (OtherBodyIndex :type Integer))
  (if (== OtherActor (Game|GetPlayerCharacter 0))
    (Variables|Default|SetPlayerRef 0)
    (Class|KismetSystemLibrary|PauseTimer 0 "ShootProjectile")
    (Utilities|Time|PauseTimerbyHandle (Variables|Default|GetLookEventTimeHandle))))

(event Custom|LookCooldown
  (Utilities|FlowControl|Delay 0.2)
  (Variables|Default|SetIsShooting false))

(event Custom|LookAtPlayer
  (Variables|Default|GetPlayerRef
    (:then
      (Variables|Default|GetIsShooting
        (:then)
        (:else
          (Transformation|SetWorldRotation (Variables|Default|GetCylinder) (Math|Rotator|MakeRotator 0.0 0.0 (.Yaw (Math|Rotator|BreakRotator (Math|Rotator|FindLookatRotation (Transformation|GetWorldLocation (Variables|Default|GetCylinder)) (Transformation|GetWorldLocation (Variables|/Script/Engine.Character|GetCapsuleComponent (Variables|Default|GetPlayerRef))))))) false false))))
    (:else)))

(event EventBeginPlay
  (bind _asabp_corn (Utilities|Casting|CastToABP_Corn (Components|SkeletalMesh|GetAnimInstance (Variables|Default|GetSkeletalMesh))))
  (Variables|Default|SetABPCornRef _asabp_corn))

(fn ConstructionScript
  (|CallParentFunction))

(fn ShootProjectile
  (bind _projectilespawn (Variables|Default|GetProjectileSpawn))
  (bind _returnvalue (Transformation|GetWorldRotation _projectilespawn))
  (bind (_roll _pitch _yaw) (Math|Rotator|BreakRotator _returnvalue))
  (Variables|Default|GetPlayerRef
    (:then
      (Audio|PlaySound2D "/Game/Assets/Sound/SFX/MutantPlants/Corn/SC_CornShooting.SC_CornShooting" 1.0 1.0 0.0 0 0)
      (Game|SpawnActorfromClass (Variables|Default|GetProjectileClassRef) (Math|Transform|MakeTransform (Transformation|GetWorldLocation _projectilespawn) (Math|Rotator|MakeRotator _roll _pitch (+ _yaw (Math|Float|Clamp(Float) (Math|Random|RandomFloat) -5e+01 5e+01))) "1.000000,1.000000,1.000000") "Undefined" "MultiplyWithRoot" 0 0))
    (:else)))

(fn BeginShootAnim
  (Variables|Default|SetIsShooting true)
  (Animation|Montage|MontagePlay (Variables|Default|GetABPCornRef) "/Game/Assets/Meshes/Plants/Mais/AM_CornShoot.AM_CornShoot" 1.0 "MontageLength" 0.0 true))