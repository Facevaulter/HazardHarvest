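; BP_CabbageShockwave is a short-lived expanding shockwave for the cabbage mutant plant that stuns players it reaches.
; On BeginPlay a timeline, with play rate set to the inverse of PlayrateTimeline, widens the pivot toward MaxScale with flattened height and grows the collision sphere alongside it.
; Players overlapping the sphere get Stunned for StunDuration.
; The actor destroys itself when the timeline finishes.
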(event OnComponentBeginOverlap(Sphere)
  (params (OverlappedComponent :type Primitive%20Component%20Object%20Reference) (OtherActor :type Actor%20Object%20Reference) (OtherComp :type Primitive%20Component%20Object%20Reference) (OtherBodyIndex :type Integer) (bFromSweep :type Boolean) (SweepResult :type Hit%20Result%20Structure%20%28by%20ref%29))
  (bind _asbp_player (Utilities|Casting|CastToBP_Player OtherActor))
  (Default|Stunned _asbp_player (Variables|Default|GetStun%20Duration)))

(event EventBeginPlay
  (bind _maxscale (Variables|Default|GetmaxScale))
  (Components|Timeline|SetPlayRate (Variables|Default|GetTimeline) (/ 1.0 (Variables|Default|GetPlayrateTimeline)))
  (bind _newtrack_0 (Timeline|Timeline PlayFromStart)
    (:Update
      (Transformation|SetRelativeScale3D (Variables|Default|GetScalingPivot) (Math|Vector|MakeVector (* _newtrack_0 _maxscale) (* _newtrack_0 _maxscale) (* _newtrack_0 0.3)))
      (Components|Sphere|SetSphereRadius (Variables|Default|GetSphere) (* _newtrack_0 (+ (* (Variables|Default|GetmaxScale) 1e+02) 2e+01)) true))
    (:Finished
      (Actor|DestroyActor))))

(fn ConstructionScript)