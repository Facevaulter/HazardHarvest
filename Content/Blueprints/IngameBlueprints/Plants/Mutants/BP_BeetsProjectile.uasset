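; Beetroot projectile, from the mutant plants set, that tracks the player from high overhead, then falls and stuns on impact.
; A fast looping timer keeps it above the player and moves a ground shadow beneath them, faded in by a timeline on a dynamic material.
; After the tracking time it pauses, then a timeline drops the sphere.
; Impact plays a splash, stuns the player if inside the overlap radius, and destroys the actor.
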(event Custom|UpdateTracking
  (bind _playerref (Variables|Default|GetPlayerRef))
  (bind _returnvalue (Transformation|GetActorLocation _playerref))
  (bind (_x _y _z) (Math|Vector|BreakVector _returnvalue))
  (if (Utilities|Enum|Equal(Enum) (Variables|Default|GetCurrentState) "NewEnumerator1")
    (Transformation|SetActorLocation (Math|Vector|MakeVector _x _y (+ _z 4e+03)) false false)
    (Transformation|SetWorldLocation (Variables|Default|GetImpactShadow) (Math|Vector|MakeVector _x _y (- _z 9e+01)) false false)
    (bind _shadowalpha (Timeline|ShadowFadeIn Play)
      (:Update
        (Rendering|Material|SetScalarParameterValueonMaterials (Variables|Default|GetImpactShadow) "ShadowOpacity" (Math|Float|Lerp 0.0 0.7 _shadowalpha))
        (Utilities|FlowControl|Delay (Variables|Default|GetTrackTime))
        (Utilities|Time|PauseTimerbyHandle (Variables|Default|GetTrackingTimeHandle))
        (CallFunction|ProjectileDrop)))))

(event Custom|ProjectileDrop
  (bind _sphere (Variables|Default|GetSphere))
  (bind _returnvalue (Transformation|GetWorldLocation _sphere))
  (bind (_x _y _z) (Math|Vector|BreakVector _returnvalue))
  (Variables|Default|SetCurrentState "NewEnumerator0")
  (Utilities|FlowControl|Delay (Variables|Default|GetDropDelay))
  (bind _alpha (Timeline|DropAnim Play)
    (:Update
      (Transformation|SetWorldLocation (Variables|Default|GetSphere) (Math|Vector|MakeVector _x _y (Math|Float|Lerp _z 0.0 _alpha)) false false))
    (:Finished
      (CallFunction|Impact))))

(event Custom|Impact
  (Audio|PlaySound2D "/Game/Assets/Sound/SFX/MutantPlants/Beetroot/SC_Beetroot_Splash.SC_Beetroot_Splash" 1.0 1.0 0.0 0 0)
  (bind _returnvalue (Collision|SphereOverlapActors (Transformation|GetWorldLocation (Variables|Default|GetSphere)) 2e+02 (Utilities|Array|MakeArray "ObjectTypeQuery3") "/Game/Blueprints/Core/BP_Player.BP_Player_C"))
  (if _returnvalue
    (Default|Stunned (Variables|Default|GetPlayerRef) (Variables|Default|GetStun%20Duration)))
  (Utilities|IsValid self
    (:Is%20Valid
      (Actor|DestroyActor))))

(event EventBeginPlay
  (bind _asbp_player (Utilities|Casting|CastToBP_Player (Game|GetPlayerCharacter 0)))
  (Variables|Default|SetPlayerRef _asbp_player)
  (bind _returnvalue (Rendering|Material|CreateDynamicMaterialInstance "/Game/Materials/M_ImpactShadow.M_ImpactShadow" "None" "None" :!class /Script/Engine.KismetMaterialLibrary))
  (bind _output_get (Variables|Default|SetImpactShadowMaterial _returnvalue))
  (Rendering|Material|SetMaterial (Variables|Default|GetImpactShadow) 0 _output_get)
  (bind _returnvalue_2 (Utilities|Time|SetTimerbyEvent (delegate Custom|UpdateTracking) 0.01 true))
  (Variables|Default|SetTrackingTimeHandle _returnvalue_2))

(fn ConstructionScript)