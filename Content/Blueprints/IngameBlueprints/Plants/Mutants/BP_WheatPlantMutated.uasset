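; BP_WheatPlantMutated is a mutated wheat plant that acts as a trap, snatching and stunning the player.
; When the player enters its Box, Trap triggers the ABP_Wheat catch event, plays a snatch sound and calls Stunned on BP_Player for SlowDuration.
; It also snaps the player's capsule to the PlayerPull point horizontally, keeping its height.
; An Activated flag blocks retriggering until Reset clears it after ResetDuration.
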(event OnComponentBeginOverlap(Box)
  (params (OverlappedComponent :type Primitive%20Component%20Object%20Reference) (OtherActor :type Actor%20Object%20Reference) (OtherComp :type Primitive%20Component%20Object%20Reference) (OtherBodyIndex :type Integer) (bFromSweep :type Boolean) (SweepResult :type Hit%20Result%20Structure%20%28by%20ref%29))
  (if (== OtherActor (Game|GetPlayerCharacter 0))
    (if (not (Variables|Default|GetActivated?))
      (CallFunction|Trap))))

(event OnComponentEndOverlap(Box)
  (params (OverlappedComponent :type Primitive%20Component%20Object%20Reference) (OtherActor :type Actor%20Object%20Reference) (OtherComp :type Primitive%20Component%20Object%20Reference) (OtherBodyIndex :type Integer)))

(event Custom|Reset
  (Utilities|FlowControl|Delay (Variables|Default|GetResetDuration))
  (Variables|Default|SetActivated? false))

(event EventBeginPlay
  (bind _asabp_wheat (Utilities|Casting|CastToABP_Wheat (Components|SkeletalMesh|GetAnimInstance (Variables|Default|GetSkeletalMesh))))
  (Variables|Default|SetABPWheatRef _asabp_wheat))

(fn ConstructionScript
  (|CallParentFunction))

(fn Trap
  (bind _playerpull (Variables|Default|GetPlayerPull))
  (bind _returnvalue (Transformation|GetWorldLocation _playerpull))
  (bind (_x _y) (Math|Vector|BreakVector _returnvalue))
  (Default|CatchEvent (Variables|Default|GetABPWheatRef) (Variables|Default|GetSlowDuration))
  (Audio|PlaySound2D "/Game/Assets/Sound/SFX/MutantPlants/Wheat/SC_WheatSnatch.SC_WheatSnatch" 1.0 1.0 0.0 0 0)
  (Variables|Default|SetActivated? true)
  (bind _asbp_player (Utilities|Casting|CastToBP_Player (Game|GetPlayerCharacter 0)))
  (Default|Stunned _asbp_player (Variables|Default|GetSlowDuration))
  (Transformation|SetWorldLocation (Variables|/Script/Engine.Character|GetCapsuleComponent _asbp_player) (Math|Vector|MakeVector _x _y (.Z (Math|Vector|BreakVector (Transformation|GetWorldLocation (Variables|/Script/Engine.Character|GetCapsuleComponent _asbp_player))))) false false)
  (CallFunction|Reset))