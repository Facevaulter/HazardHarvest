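; Tomato mutant enemy character that chases the player, explodes to stun them, and destroys itself when day begins.
; A timeline spins its pivot in pitch, while entering the aggro trigger starts an AIMoveTo toward the player and leaving it clears the target.
; On arrival it stops, waits briefly, then explodes, stunning the player only if inside the explosion radius.
; The day-start cleanup is bound through BP_DayNightManager's dispatcher.
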(event OnComponentBeginOverlap(ExplosionRadius)
  (params (OverlappedComponent :type Primitive%20Component%20Object%20Reference) (OtherActor :type Actor%20Object%20Reference) (OtherComp :type Primitive%20Component%20Object%20Reference) (OtherBodyIndex :type Integer) (bFromSweep :type Boolean) (SweepResult :type Hit%20Result%20Structure%20%28by%20ref%29))
  (if (== OtherActor (Game|GetPlayerCharacter 0))
    (Variables|Default|SetInExplosionRadius true)))

(event OnComponentEndOverlap(ExplosionRadius)
  (params (OverlappedComponent :type Primitive%20Component%20Object%20Reference) (OtherActor :type Actor%20Object%20Reference) (OtherComp :type Primitive%20Component%20Object%20Reference) (OtherBodyIndex :type Integer))
  (if (== OtherActor (Game|GetPlayerCharacter 0))
    (Variables|Default|SetInExplosionRadius false)))

(event OnComponentBeginOverlap(AggroTrigger)
  (params (OverlappedComponent :type Primitive%20Component%20Object%20Reference) (OtherActor :type Actor%20Object%20Reference) (OtherComp :type Primitive%20Component%20Object%20Reference) (OtherBodyIndex :type Integer) (bFromSweep :type Boolean) (SweepResult :type Hit%20Result%20Structure%20%28by%20ref%29))
  (if (== OtherActor (Game|GetPlayerCharacter 0))
    (bind _returnvalue (Actor|GetActorOfClass "/Game/Blueprints/Core/BP_Player.BP_Player_C"))
    (Variables|Default|SetPlayerRef _returnvalue)
    (CallFunction|SearchTarget)))

(event OnComponentEndOverlap(AggroTrigger)
  (params (OverlappedComponent :type Primitive%20Component%20Object%20Reference) (OtherActor :type Actor%20Object%20Reference) (OtherComp :type Primitive%20Component%20Object%20Reference) (OtherBodyIndex :type Integer))
  (if (== OtherActor (Game|GetPlayerCharacter 0))
    (Variables|Default|SetPlayerRef 0)
    (Components|Movement|StopMovementImmediately (Variables|Character|GetCharacterMovement))))

(event Custom|DestroyOnDay
  (Utilities|IsValid self
    (:Is%20Valid
      (EventDispatchers|UnbindEventfromBeginDayDispatcher (stale EventBeginPlay _output_get) (delegate Custom|DestroyOnDay))
      (Actor|DestroyActor))))

(event Custom|Explode
  (Default|CallTomatoExplosion)
  (if (Variables|Default|GetInExplosionRadius)
    (Default|Stunned (Variables|Default|GetPlayerRef) (Variables|Default|GetStunDuration)))
  (Utilities|IsValid self
    (:Is%20Valid
      (Actor|DestroyActor))))

(event Custom|StartRotating
  (Timeline|RotationTimeline PlayFromStart
    (:Update
      (Transformation|AddLocalRotation (Variables|Default|GetRotationPivot) (Math|Rotator|MakeRotator 0.0 (Variables|Default|GetRotationSpeed) 0.0) false false))))

(event Custom|SearchTarget
  (bind _playerref (Variables|Default|GetPlayerRef))
  (Utilities|FlowControl|Delay 0.05)
  (AI|AIMoveTo self (Transformation|GetActorLocation _playerref) _playerref (Variables|/Script/Engine.SphereComponent|GetSphereRadius (Variables|Default|GetExplosionTrigger)) false
    (:OnSuccess
      (Components|Movement|StopMovementImmediately (Variables|Character|GetCharacterMovement))
      (CallFunction|StopRotating)
      (Utilities|FlowControl|Delay 1.0)
      (CallFunction|Explode))))

(event Custom|StopRotating
  (Timeline|RotationTimeline Stop
    (:Update
      (Transformation|AddLocalRotation (Variables|Default|GetRotationPivot) (Math|Rotator|MakeRotator 0.0 (Variables|Default|GetRotationSpeed) 0.0) false false))))

(event EventBeginPlay
  (bind _returnvalue (Actor|GetActorOfClass "/Game/Blueprints/IngameBlueprints/BP_DayNightManager.BP_DayNightManager_C"))
  (bind _output_get (Variables|Default|SetDayNightManagerRef _returnvalue))
  (EventDispatchers|BindEventtoBeginDayDispatcher _output_get (delegate Custom|DestroyOnDay))
  (Components|Timeline|SetPlayRate (Variables|Default|GetRotationTimeline) (/ 1.0 (Variables|Default|GetRotationTimelinePlayRate)))
  (CallFunction|StartRotating))

(fn ConstructionScript)