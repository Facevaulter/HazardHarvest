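; Mutant pumpkin plant enemy that turns toward the player and repeatedly attacks in a straight line, stunning on hit.
; Aggro range overlap starts a looping look-at timer, which holds rotation during attacks.
; Attack range overlap drives a delay-based loop: Niagara telegraph sized to attack width, then montage, with montage length as the attacking window.
; HitCheck, called from outside this graph, sphere-traces forward and stuns the player.
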(event OnComponentBeginOverlap(AttackRange)
  (params (OverlappedComponent :type Primitive%20Component%20Object%20Reference) (OtherActor :type Actor%20Object%20Reference) (OtherComp :type Primitive%20Component%20Object%20Reference) (OtherBodyIndex :type Integer) (bFromSweep :type Boolean) (SweepResult :type Hit%20Result%20Structure%20%28by%20ref%29))
  (bind _attackinterval (Variables|Default|GetAttackInterval))
  (if (== OtherActor (Game|GetPlayerCharacter 0))
    (Variables|Default|SetCanAttack true)
    (Variables|Default|GetIsInAttackLoop
      (:then)
      (:else
        (Variables|Default|SetIsInAttackLoop true)
        (|AktivateAttackTelegraph_2_2 _attackinterval)
        (Utilities|FlowControl|Delay _attackinterval)
        (CallFunction|TryAttack)))))

(event OnComponentBeginOverlap(AggroRange)
  (params (OverlappedComponent :type Primitive%20Component%20Object%20Reference) (OtherActor :type Actor%20Object%20Reference) (OtherComp :type Primitive%20Component%20Object%20Reference) (OtherBodyIndex :type Integer) (bFromSweep :type Boolean) (SweepResult :type Hit%20Result%20Structure%20%28by%20ref%29))
  (bind _returnvalue (Game|GetPlayerCharacter 0))
  (if (== OtherActor _returnvalue)
    (bind _asbp_player (Utilities|Casting|CastToBP_Player _returnvalue))
    (Variables|Default|SetPlayerRef _asbp_player)
    (bind _returnvalue_2 (Utilities|Time|SetTimerbyEvent (delegate Custom|LookAtPlayer) 0.02 true))
    (Variables|Default|SetLookEventTimerHandle _returnvalue_2)))

(event OnComponentEndOverlap(AttackRange)
  (params (OverlappedComponent :type Primitive%20Component%20Object%20Reference) (OtherActor :type Actor%20Object%20Reference) (OtherComp :type Primitive%20Component%20Object%20Reference) (OtherBodyIndex :type Integer))
  (if (== OtherActor (Game|GetPlayerCharacter 0))
    (Variables|Default|SetCanAttack false)))

(event OnComponentEndOverlap(AggroRange)
  (params (OverlappedComponent :type Primitive%20Component%20Object%20Reference) (OtherActor :type Actor%20Object%20Reference) (OtherComp :type Primitive%20Component%20Object%20Reference) (OtherBodyIndex :type Integer))
  (if (== OtherActor (Game|GetPlayerCharacter 0))
    (Variables|Default|SetPlayerRef 0)
    (Class|KismetSystemLibrary|PauseTimer 0 "TryAttack")
    (Utilities|Time|PauseTimerbyHandle (Variables|Default|GetLookEventTimerHandle))))

(event Custom|SuccessfulHit
  (Default|Stunned (Variables|Default|GetPlayerRef) (Variables|Default|GetStunDuration)))

(event Custom|LookAtPlayer
  (Variables|Default|GetIsAttacking
    (:then)
    (:else
      (Variables|Default|GetPlayerRef
        (:then
          (Transformation|SetWorldRotation (Variables|Default|GetSphere) (Math|Rotator|MakeRotator 0.0 0.0 (.Yaw (Math|Rotator|BreakRotator (Math|Rotator|FindLookatRotation (Transformation|GetWorldLocation (Variables|Default|GetSkeletalMesh)) (Transformation|GetWorldLocation (Variables|/Script/Engine.Character|GetCapsuleComponent (Variables|Default|GetPlayerRef))))))) false false))
        (:else)))))

(event Custom|HitCheck
  (bind _returnvalue (Transformation|GetActorLocation))
  (bind _returnvalue_2 (+ _returnvalue "0.000000,0.000000,100.000000"))
  (Audio|PlaySound2D "/Game/Assets/Sound/SFX/MutantPlants/Pumpkin/SC_PumpkinAttack.SC_PumpkinAttack" 1.0 1.0 0.0 0 0)
  (bind _outhits (Collision|MultiSphereTraceByChannel _returnvalue_2 (+ _returnvalue_2 (* (Math|Vector|GetForwardVector (Variables|Default|GetForward)) "330.000000,330.000000,330.000000")) (Variables|Default|GetAttackWidth) "TraceTypeQuery1" false 0 "None"))
  (for _array_element _outhits
    (Utilities|Casting|CastToBP_Player (.HitActor (Collision|BreakHitResult _array_element)))
    (CallFunction|SuccessfulHit)))

(event Custom|AttackCooldown
  (params (Duration :type Float%20%28single-precision%29))
  (Variables|Default|SetIsAttacking true)
  (Utilities|FlowControl|Delay Duration)
  (Variables|Default|SetIsAttacking false))

(event Custom|LoopAttack
  (bind _attackinterval (Variables|Default|GetAttackInterval))
  (Variables|Default|GetCanAttack
    (:then
      (Variables|Default|SetIsInAttackLoop true)
      (|AktivateAttackTelegraph_2_2 _attackinterval)
      (Utilities|FlowControl|Delay _attackinterval)
      (CallFunction|TryAttack))
    (:else
      (Variables|Default|SetIsInAttackLoop false))))

(event EventBeginPlay
  (bind _asabp_pumpkin (Utilities|Casting|CastToABP_Pumpkin (Components|SkeletalMesh|GetAnimInstance (Variables|Default|GetSkeletalMesh))))
  (Variables|Default|SetABPPumpkinRef _asabp_pumpkin))

(fn ConstructionScript
  (|CallParentFunction))

(fn TryAttack
  (bind _returnvalue (Animation|Montage|MontagePlay (Variables|Default|GetABPPumpkinRef) "/Game/Assets/Meshes/Plants/Kürbis/AM_PumpkinAttack.AM_PumpkinAttack" 1.0 "MontageLength" 0.0 true))
  (CallFunction|AttackCooldown _returnvalue)
  (CallFunction|LoopAttack))