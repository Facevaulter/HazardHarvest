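; BP_TomatoPlantMutant is a mutant tomato plant that turns into an enemy character when the player gets close.
; The first time the player character overlaps AggroTrigger, it hides itself and spawns BP_TomatoMutantCharacter at the Sphere component's transform.
; It then calls MutantOnTheLoose and sets IsActivated so the swap happens only once.
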(event OnComponentBeginOverlap(AggroTrigger)
  (params (OverlappedComponent :type Primitive%20Component%20Object%20Reference) (OtherActor :type Actor%20Object%20Reference) (OtherComp :type Primitive%20Component%20Object%20Reference) (OtherBodyIndex :type Integer) (bFromSweep :type Boolean) (SweepResult :type Hit%20Result%20Structure%20%28by%20ref%29))
  (if (== OtherActor (Game|GetPlayerCharacter 0))
    (if (not (Variables|Default|GetIsActivated?))
      (Rendering|SetActorHiddenInGame true)
      (Game|SpawnActorfromClass "/Game/Blueprints/IngameBlueprints/Plants/Mutants/BP_TomatoMutantCharacter.BP_TomatoMutantCharacter_C" (Transformation|GetWorldTransform (Variables|Default|GetSphere)) "Undefined" "MultiplyWithRoot" 0 0)
      (Default|CallMutantontheLoose)
      (Variables|Default|SetIsActivated? true))))

(fn ConstructionScript
  (|CallParentFunction))