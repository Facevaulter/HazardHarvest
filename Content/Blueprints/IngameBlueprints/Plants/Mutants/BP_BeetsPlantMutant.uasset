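; Beet mutant plant enemy that turns to face the player inside its aggro range and makes mortar-style attacks.
; Range overlap starts looping timers for yaw tracking and an attack montage, and leaving pauses both.
; A separate SpawnProjectile event, not called by live logic here, fires an upward projectile, then after a delay spawns mini radishes high above the player's current position.
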(event OnComponentBeginOverlap(AggroRange)
  (params (OverlappedComponent :type Primitive%20Component%20Object%20Reference) (OtherActor :type Actor%20Object%20Reference) (OtherComp :type Primitive%20Component%20Object%20Reference) (OtherBodyIndex :type Integer) (bFromSweep :type Boolean) (SweepResult :type Hit%20Result%20Structure%20%28by%20ref%29))
  (bind _returnvalue (Game|GetPlayerCharacter 0))
  (if (== OtherActor _returnvalue)
    (bind _asbp_player (Utilities|Casting|CastToBP_Player _returnvalue))
    (Variables|Default|SetPlayerRef _asbp_player)
    (bind _returnvalue_2 (Utilities|Time|SetTimerbyEvent (delegate Custom|LookAtPlayer) 0.01 true))
    (Variables|Default|SetLookEventTimeHandle _returnvalue_2)
    (CallFunction|ShootProjectile)
    (Utilities|Time|SetTimerbyFunctionName 0 "ShootProjectile" (Variables|Default|GetAttackInterval) true)))

(event OnComponentEndOverlap(AggroRange)
  (params (OverlappedComponent :type Primitive%20Component%20Object%20Reference) (OtherActor :type Actor%20Object%20Reference) (OtherComp :type Primitive%20Component%20Object%20Reference) (OtherBodyIndex :type Integer))
  (if (== OtherActor (Game|GetPlayerCharacter 0))
    (Variables|Default|SetPlayerRef 0)
    (Class|KismetSystemLibrary|PauseTimer 0 "ShootProjectile")
    (Utilities|Time|PauseTimerbyHandle (Variables|Default|GetLookEventTimeHandle))))

(event Custom|SpawnProjectile
  (bind _playerref (Variables|Default|GetPlayerRef))
  (bind _capsulecomponent (Variables|/Script/Engine.Character|GetCapsuleComponent _playerref))
  (bind _returnvalue (Transformation|GetWorldLocation _capsulecomponent))
  (bind (_x _y) (Math|Vector|BreakVector _returnvalue))
  (Audio|PlaySound2D "/Game/Assets/Sound/SFX/MutantPlants/Beetroot/SC_Beetroot_Attack.SC_Beetroot_Attack" 1.0 1.0 0.0 0 0)
  (Game|SpawnActorfromClass "/Game/Blueprints/IngameBlueprints/Plants/Mutants/BP_BeetsProjectileUP.BP_BeetsProjectileUP_C" (Transformation|GetWorldTransform (Variables|Default|GetProjectileSpawn)) "Undefined" "MultiplyWithRoot" 0 0)
  (Utilities|FlowControl|Delay 2.0)
  (Game|SpawnActorfromClass (Variables|Default|GetMiniRadishesClassRef) (Math|Transform|MakeTransform (Math|Vector|MakeVector _x _y 4e+03) "0, 0, 0" "1.000000,1.000000,1.000000") "Undefined" "MultiplyWithRoot" 0 0))

(event Custom|LookAtPlayer
  (Variables|Default|GetPlayerRef
    (:then
      (Transformation|SetWorldRotation (Variables|Default|GetSkeletalMesh) (Math|Rotator|MakeRotator 0.0 0.0 (.Yaw (Math|Rotator|BreakRotator (Math|Rotator|FindLookatRotation (Transformation|GetWorldLocation (Variables|Default|GetSkeletalMesh)) (Transformation|GetWorldLocation (Variables|/Script/Engine.Character|GetCapsuleComponent (Variables|Default|GetPlayerRef))))))) false false))
    (:else)))

(event EventBeginPlay
  (bind _asabp_beets (Utilities|Casting|CastToABP_Beets (Components|SkeletalMesh|GetAnimInstance (Variables|Default|GetSkeletalMesh))))
  (Variables|Default|SetAnimBPRef _asabp_beets)
  (bind _asbp_player (Utilities|Casting|CastToBP_Player (Game|GetPlayerCharacter 0)))
  (Variables|Default|SetPlayerRef _asbp_player))

(fn ConstructionScript
  (|CallParentFunction))

(fn ShootProjectile
  (Variables|Default|GetPlayerRef
    (:then
      (Animation|Montage|MontagePlay (Variables|Default|GetAnimBPRef) "/Game/Assets/Meshes/Plants/RoteBeete/AM_BeetAttack.AM_BeetAttack" 1.0 "MontageLength" 0.0 true))
    (:else)))