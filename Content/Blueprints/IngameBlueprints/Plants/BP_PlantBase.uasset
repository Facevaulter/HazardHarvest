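; Base plant actor for a farming system, handling growth, mutation, harvesting and destruction on its farm spot.
; Grow and Mutate look up the plant's ID in a data table, spawn the grown or mutated class and update the spot's plant reference.
; TryMutate only sets the Mutated flag from a random roll against the row's rate.
; Harvest clears the spot, Destroy calls PlantDestroyed, and MutationBehavior is an empty hook.
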(fn ConstructionScript)

(fn Grow
  (bind _bp_farmspotref (Variables|Default|GetBP_FarmSpotRef))
  (Utilities|IsValid self
    (:Is%20Valid
      (Utilities|IsValid (Variables|/Game/Blueprints/IngameBlueprints/FarmSpots/BP_CropPlotBase.BP_CropPlotBase_C|GetCurrentPlant (Variables|Default|GetBP_FarmSpotRef))
        (:Is%20Valid
          (Actor|DestroyActor (Variables|/Game/Blueprints/IngameBlueprints/FarmSpots/BP_CropPlotBase.BP_CropPlotBase_C|GetCurrentPlant (Variables|Default|GetBP_FarmSpotRef)))
          (bind _returnvalue (Utilities|GetDataTableRow (Variables|Default|GetPlantData) (Variables|Default|GetID))
            (:then
              (bind _returnvalue_2 (Game|SpawnActorfromClass (.GrownPlantClass (Utilities|Struct|BreakST_PlantData _returnvalue)) (Transformation|GetWorldTransform (Variables|/Game/Blueprints/IngameBlueprints/FarmSpots/BP_CropPlotBase.BP_CropPlotBase_C|GetSpawnRoot _bp_farmspotref)) "Undefined" "MultiplyWithRoot" 0 0))
              (bind _asbp_plant_base (Utilities|Casting|CastToBP_PlantBase _returnvalue_2))
              (Variables|/Game/Blueprints/IngameBlueprints/FarmSpots/BP_CropPlotBase.BP_CropPlotBase_C|SetCurrentPlant _bp_farmspotref _asbp_plant_base)
              (Variables|/Game/Blueprints/IngameBlueprints/FarmSpots/BP_CropPlotBase.BP_CropPlotBase_C|SetCurrentPlantID _bp_farmspotref (.PlantID (Utilities|Struct|BreakST_PlantData _returnvalue)))
              (Variables|Default|SetHarvestable? true)
              (Variables|Default|SetGoldMultiplier 1.0))))))))

(fn Mutate
  (bind _bp_farmspotref (Variables|Default|GetBP_FarmSpotRef))
  (bind _bp_farmspotref_2 (Variables|Default|GetBP_FarmSpotRef))
  (Utilities|IsValid self
    (:Is%20Valid
      (bind _returnvalue (Utilities|GetDataTableRow (Variables|Default|GetPlantData) (Variables|Default|GetID))
        (:then
          (if (Utilities|IsValidClass (.MutatedClass (Utilities|Struct|BreakST_PlantData _returnvalue)))
            (Utilities|IsValid (Variables|/Game/Blueprints/IngameBlueprints/FarmSpots/BP_CropPlotBase.BP_CropPlotBase_C|GetCurrentPlant _bp_farmspotref)
              (:Is%20Valid
                (bind _returnvalue_2 (Game|SpawnActorfromClass (.MutatedClass (Utilities|Struct|BreakST_PlantData _returnvalue)) (Transformation|GetWorldTransform (Variables|/Game/Blueprints/IngameBlueprints/FarmSpots/BP_CropPlotBase.BP_CropPlotBase_C|GetSpawnRoot _bp_farmspotref)) "Undefined" "MultiplyWithRoot" 0 0))
                (bind _asbp_plant_base (Utilities|Casting|CastToBP_PlantBase _returnvalue_2))
                (bind _output_get (Variables|/Game/Blueprints/IngameBlueprints/FarmSpots/BP_CropPlotBase.BP_CropPlotBase_C|SetCurrentPlant _bp_farmspotref_2 _asbp_plant_base))
                (Variables|/Game/Blueprints/IngameBlueprints/FarmSpots/BP_CropPlotBase.BP_CropPlotBase_C|SetCurrentPlantID _bp_farmspotref_2 (.PlantID (Utilities|Struct|BreakST_PlantData _returnvalue)))
                (Variables|BP_PlantBase_C|SetCanBeBugTarget _output_get false)
                (Actor|DestroyActor (Variables|/Game/Blueprints/IngameBlueprints/FarmSpots/BP_CropPlotBase.BP_CropPlotBase_C|GetCurrentPlant _bp_farmspotref))))))))))

(fn TryMutate
  (Utilities|IsValid self
    (:Is%20Valid
      (bind _returnvalue (Utilities|GetDataTableRow (Variables|Default|GetPlantData) (Variables|Default|GetID))
        (:then
          (if (<= (Math|Float|Clamp(Float) (Math|Random|RandomFloat)) (.MutationRate (Utilities|Struct|BreakST_PlantData _returnvalue)))
            (Variables|Default|SetMutated? true)))))))

(fn Harvest
  (bind _bp_farmspotref (Variables|Default|GetBP_FarmSpotRef))
  (Utilities|IsValid self
    (:Is%20Valid
      (if (Variables|Default|GetHarvestable?)
        (Utilities|IsValid (Variables|/Game/Blueprints/IngameBlueprints/FarmSpots/BP_CropPlotBase.BP_CropPlotBase_C|GetCurrentPlant _bp_farmspotref)
          (:Is%20Valid
            (Actor|DestroyActor (Variables|/Game/Blueprints/IngameBlueprints/FarmSpots/BP_CropPlotBase.BP_CropPlotBase_C|GetCurrentPlant _bp_farmspotref))
            (Variables|/Game/Blueprints/IngameBlueprints/FarmSpots/BP_CropPlotBase.BP_CropPlotBase_C|SetCurrentPlant _bp_farmspotref 0)
            (Variables|/Game/Blueprints/IngameBlueprints/FarmSpots/BP_CropPlotBase.BP_CropPlotBase_C|SetCurrentPlantID _bp_farmspotref "None")
            (Variables|Default|SetHarvestable? false)))))))

(fn Destroy
  (Utilities|IsValid self
    (:Is%20Valid
      (Variables|Default|SetDestroyed? true)
      (Default|CallPlantDestroyed)
      (Actor|DestroyActor))))

(fn MutationBehavior)