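; Manager that drives the farming day/night cycle, switching sun angle, atmosphere, UI, interactables and crop plot state.
; BeginNight grows every plant, shuffles mutation candidates to mutate some, and starts a looping timer spawning bugs at spawn points.
; BugKilled triggers BeginDay once the nightly kill quota is reached.
; BeginDay harvests plants into player inventory, shows night results, clears night state and randomly reserves a percentage of plots as fertilized.
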(event Custom|SetSpawnPoints
  (bind _outactors (Actor|GetAllActorsOfClass "/Game/Blueprints/IngameBlueprints/BugSystem/BP_BugSpawnPoint.BP_BugSpawnPoint_C"))
  (for _array_element _outactors
    (Utilities|Array|Add (Variables|Default|GetSpawnPoints) _array_element)))

(event EventBeginPlay
  (bind _asbp_player (Utilities|Casting|CastToBP_Player (Game|GetPlayerCharacter 0)))
  (Variables|Default|SetPlayerRef _asbp_player))

(fn ConstructionScript)

(fn BeginNight
  (bind _unmutatedplants (Variables|Default|GetUnMutatedPlants))
  (bind _mutationcandidates (Variables|Default|GetMutationCandidates))
  (Default|CallBeginNightDispatcher)
  (bind _asbp_player (Utilities|Casting|CastToBP_Player (Game|GetPlayerCharacter 0)))
  (Variables|/Game/Blueprints/Core/BP_Player.BP_Player_C|SetIsNight _asbp_player true)
  (Default|PlayNightAtmo _asbp_player)
  (for _array_element (Variables|Default|GetActorsToToggleInteract)
    (Class|BPIInteract|SetInteractStatus(Message) _array_element false))
  (|ChangeUitoNight)
  (Variables|Default|SetIsNight? true)
  (Transformation|SetActorRelativeRotation (Variables|Default|GetSunRef) "-177.000000,0.000000,0.000000")
  (Utilities|Array|Clear (Variables|Default|GetFertileCandidates))
  (Variables|Default|SetTotalCandidateCrops 0)
  (CallFunction|SetSpawnPoints)
  (Utilities|Time|SetTimerbyFunctionName 0 "SpawnBug" (Variables|Default|GetBugSpawnInterval) true)
  (bind _outactors (Actor|GetAllActorsOfClass "/Game/Blueprints/IngameBlueprints/FarmSpots/BP_CropPlotBase.BP_CropPlotBase_C"))
  (for _array_element_2 _outactors
    (Variables|/Game/Blueprints/IngameBlueprints/FarmSpots/BP_CropPlotBase.BP_CropPlotBase_C|SetNighttime? _array_element_2 true))
  (bind _outactors_2 (Actor|GetAllActorsOfClass "/Game/Blueprints/IngameBlueprints/Plants/BP_PlantBase.BP_PlantBase_C"))
  (for _array_element_3 _outactors_2
    (Utilities|IsValid _array_element_3
      (:Is%20Valid
        (Math|Integer|IncrementInt (Variables|Default|GetTotalPlants)
          (:%20%20
            (bind _output_get (Variables|Default|SetTempFarmSpotRef (Variables|/Game/Blueprints/IngameBlueprints/Plants/BP_PlantBase.BP_PlantBase_C|GetBP_FarmSpotRef _array_element_3)))
            (bind _plantthatgrewref (Default|Grow _array_element_3))
            (bind _output_get_2 (Variables|Default|SetPlant%20That%20Grew%20Ref _plantthatgrewref))
            (Default|TryMutate _output_get_2)
            (Variables|/Game/Blueprints/IngameBlueprints/Plants/BP_PlantBase.BP_PlantBase_C|SetBP_FarmSpotRef _output_get_2 _output_get)
            (Actor|DestroyActor _array_element_3)
            (if (Variables|/Game/Blueprints/IngameBlueprints/Plants/BP_PlantBase.BP_PlantBase_C|GetMutated? _output_get_2)
              (Utilities|Array|Add (Variables|Default|GetMutationCandidates) _output_get_2)
              (else
                (Utilities|Array|Add (Variables|Default|GetUnMutatedPlants) _output_get_2))))))))
  (Utilities|Array|Shuffle (Variables|Default|GetMutationCandidates))
  (bind _output_get_3 (Variables|Default|SetMaxMutations (Math|Float|Round (* (Variables|Default|GetTotalPlants) (Variables|Default|GetMaxMutationsPercent)))))
  (for _index (range (- _output_get_3 1) (- (Utilities|Array|Length (Variables|Default|GetMutationCandidates)) 1))
    (if (Utilities|Array|IsNotEmpty _mutationcandidates)
      (if (< (Utilities|Array|Length (Variables|Default|GetMutationCandidates)) (Variables|Default|GetMinMutations))
        (Utilities|Array|Shuffle _unmutatedplants)
        (for _array_element_4 _unmutatedplants
          (Utilities|FlowControl|DoOnce false :!label _label
            (:Completed
              (Utilities|Array|Add (Variables|Default|GetMutationCandidates) _array_element_4)
              (Default|Mutate (Utilities|Array|Get(acopy) _mutationcandidates _index))
              (goto _label Reset))))
        (else
          (Default|Mutate (Utilities|Array|Get(acopy) _mutationcandidates _index))
          (Utilities|FlowControl|DoOnce false) ; enters at Reset
        )))))

(fn BeginDay
  (Default|CallBeginDayDispatcher)
  (|HarvestPlants
    (:Completed
      (bind _asbp_player (Utilities|Casting|CastToBP_Player (Game|GetPlayerCharacter 0)))
      (Variables|/Game/Blueprints/Core/BP_Player.BP_Player_C|SetIsNight _asbp_player false)
      (Default|PlayDayAtmo _asbp_player)
      (for _array_element (Variables|Default|GetActorsToToggleInteract)
        (Class|BPIInteract|SetInteractStatus(Message) _array_element true))
      (|ChangeUIToDay)
      (Variables|Default|SetIsNight? false)
      (Transformation|SetActorRelativeRotation (Variables|Default|GetSunRef) "-46.000000,0.000000,0.000000")
      (Math|Integer|IncrementInt (Variables|Default|GetDayCount)
        (:%20%20
          (CallFunction|CleanUpNight)
          (bind _outactors (Actor|GetAllActorsOfClass "/Game/Blueprints/IngameBlueprints/FarmSpots/BP_CropPlotBase.BP_CropPlotBase_C"))
          (for _array_element_2 _outactors
            (Utilities|IsValid _array_element_2
              (:Is%20Valid
                (Default|FertileReset _array_element_2)
                (Math|Integer|IncrementInt (Variables|Default|GetTotalCandidateCrops)
                  (:%20%20
                    (Utilities|IsValid (Variables|/Game/Blueprints/IngameBlueprints/FarmSpots/BP_CropPlotBase.BP_CropPlotBase_C|GetCurrentPlant _array_element_2)
                      (:Is%20Valid
                        (Variables|/Game/Blueprints/IngameBlueprints/FarmSpots/BP_CropPlotBase.BP_CropPlotBase_C|SetNighttime? _array_element_2 false))))))))
          (bind _output_get (Variables|Default|SetFertileCandidates _outactors))
          (Utilities|Array|Shuffle _output_get)
          (bind _output_get_2 (Variables|Default|SetMaxFertiledCrops (Math|Float|Round (* (Variables|Default|GetTotalCandidateCrops) (Variables|Default|GetFertileRatePercent)))))
          (for _index (range 0 (- _output_get_2 1))
            (Variables|/Game/Blueprints/IngameBlueprints/FarmSpots/BP_CropPlotBase.BP_CropPlotBase_C|SetFertilizeReserved (Utilities|Array|Get(acopy) (Variables|Default|GetFertileCandidates) _index) true)))))))

(fn BugKilled
  (Math|Integer|IncrementInt (Variables|Default|GetKilledBugs)
    (:%20%20
      (Math|Integer|DecrementInt (Variables|Default|GetCurrentBugsOnField)
        (:%20%20
          (if (>= (Variables|Default|GetKilledBugs) (Variables|Default|GetMaxBugsPerNight))
            (CallFunction|BeginDay)))))))

(fn CleanUpNight
  (Utilities|Array|Clear (Variables|Default|GetUnMutatedPlants))
  (Utilities|Array|Clear (Variables|Default|GetMutationCandidates))
  (Utilities|Array|Clear (Variables|Default|GetSpawnPoints))
  (Utilities|Array|Clear (Variables|Default|GetHarvestedCropsPlantID))
  (Utilities|Array|Clear (Variables|Default|GetHarvestedCropsAmount))
  (Variables|Default|SetCurrentBugsOnField 0)
  (Variables|Default|SetTotalPlants 0)
  (Variables|Default|SetKilledBugs 0)
  (bind _outactors (Actor|GetAllActorsOfClass "/Game/Blueprints/IngameBlueprints/BugSystem/BP_BugCharacter.BP_BugCharacter_C"))
  (for _array_element _outactors
    (Utilities|IsValid _array_element
      (:Is%20Valid
        (Actor|DestroyActor _array_element)))))

(fn SpawnBug
  (bind _returnvalue (Math|Random|RandomInteger 0))
  (bind _spawnpoints (Variables|Default|GetSpawnPoints))
  (bind _spawnpoints_2 (Variables|Default|GetSpawnPoints))
  (bind _returnvalue_2 (Utilities|Array|Length _spawnpoints_2))
  (bind _returnvalue_3 (Math|Integer|Clamp(Integer) _returnvalue 0 _returnvalue_2))
  (bind _output (Utilities|Array|Get(acopy) _spawnpoints _returnvalue_3))
  (Variables|Default|SetBugSpawnInterval (Math|Float|Clamp(Float) (Math|Random|RandomFloat) 1.0 5.0))
  (if (<= (Variables|Default|GetCurrentBugsOnField) (Variables|Default|GetMaxBugsOnField))
    (bind _outactors (Actor|GetAllActorsOfClass "/Game/Blueprints/IngameBlueprints/Plants/BP_PlantBase.BP_PlantBase_C"))
    (for _array_element _outactors
      _)
    (if (> (Utilities|Array|Length _outactors) 0)
      (Math|Integer|IncrementInt (Variables|Default|GetCurrentBugsOnField)
        (:%20%20
          (Utilities|Array|Shuffle _spawnpoints)
          (Utilities|IsValid _output
            (:Is%20Valid
              (bind _returnvalue_4 (Game|SpawnActorfromClass "/Game/Blueprints/IngameBlueprints/BugSystem/BP_BugCharacter.BP_BugCharacter_C" (Transformation|GetActorTransform _output) "Undefined" "MultiplyWithRoot" 0 0))
              (Utilities|IsValid _returnvalue_4
                (:Is%20Valid
                  (Default|SearchTarget _returnvalue_4))))))))))

(fn HarvestPlant
  (params (PlantToHarvest :type BP%20Plant%20Base%20Object%20Reference))
  (bind _id (Variables|/Game/Blueprints/IngameBlueprints/Plants/BP_PlantBase.BP_PlantBase_C|GetID PlantToHarvest))
  (bind _id_2 (Variables|/Game/Blueprints/IngameBlueprints/Plants/BP_PlantBase.BP_PlantBase_C|GetID PlantToHarvest))
  (bind _playerref (Variables|Default|GetPlayerRef))
  (bind _harvestedcropsplantid (Variables|Default|GetHarvestedCropsPlantID))
  (bind _cropinventoryseedid (Variables|/Game/Blueprints/Core/BP_Player.BP_Player_C|GetCropInventorySeedID _playerref))
  (Utilities|FlowControl|Sequence
    (:then_0
      (if (Utilities|Array|ContainsItem _harvestedcropsplantid _id_2)
        (Math|Integer|IncrementInt (Utilities|Array|Get(acopy) (Variables|Default|GetHarvestedCropsAmount) (Utilities|Array|FindItem _harvestedcropsplantid _id_2)))
        (else
          (Utilities|Array|Add (Variables|Default|GetHarvestedCropsPlantID) _id_2)
          (Utilities|Array|Add (Variables|Default|GetHarvestedCropsAmount) 1))))
    (:then_1
      (if (Utilities|Array|ContainsItem _cropinventoryseedid _id)
        (Math|Integer|IncrementInt (Utilities|Array|Get(acopy) (Variables|/Game/Blueprints/Core/BP_Player.BP_Player_C|GetCropCount (Variables|Default|GetPlayerRef)) (Utilities|Array|FindItem _cropinventoryseedid _id)))
        (else
          (Utilities|Array|Add (Variables|/Game/Blueprints/Core/BP_Player.BP_Player_C|GetCropInventorySeedID (Variables|Default|GetPlayerRef)) _id)
          (Utilities|Array|Add (Variables|/Game/Blueprints/Core/BP_Player.BP_Player_C|GetCropCount (Variables|Default|GetPlayerRef)) 1))))))