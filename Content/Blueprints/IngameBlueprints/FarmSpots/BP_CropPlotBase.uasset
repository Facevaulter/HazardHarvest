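; BP_CropPlotBase is the base farm plot that the player interacts with outside nighttime to plant seeds and harvest crops.
; An empty plot looks up the player's seed ID in a data table, spawns that plant as a bug-targetable actor and links it back.
; An occupied plot harvests ready plants, then either applies reserved fertilizer as a value multiplier boost or resets it.
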(event EventInteract
  (params (Sender :type Actor%20Object%20Reference))
  (bind _currentplant (Variables|Default|GetCurrentPlant))
  (if (not (Variables|Default|GetNighttime?))
    (if (Variables|Default|GetOccupied?)
      (if (Variables|/Game/Blueprints/IngameBlueprints/Plants/BP_PlantBase.BP_PlantBase_C|GetHarvestable? _currentplant)
        (Default|Harvest _currentplant)
        (Variables|Default|SetSuccessfullyPlanted? false)
        (if (Variables|Default|GetFertilizeReserved)
          (Variables|Default|SetFertilizeReserved false)
          (CallFunction|Fertiled)
          (else
            (CallFunction|FertileReset))))
      (else
        (bind _asbp_player (Utilities|Casting|CastToBP_Player Sender))
        (CallFunction|PlantSeed (Variables|/Game/Blueprints/Core/BP_Player.BP_Player_C|GetCurrentSeedID _asbp_player))
        (Variables|Default|SetSuccessfullyPlanted? true)))))

(fn ConstructionScript)

(fn PlantSeed
  (params (PlantID :type Name))
  (bind _returnvalue (Utilities|GetDataTableRow (Variables|Default|GetPlantData) PlantID)
    (:then
      (bind _returnvalue_2 (Game|SpawnActorfromClass (.PlantClass (Utilities|Struct|BreakST_PlantData _returnvalue)) (Transformation|GetWorldTransform (Variables|Default|GetSpawnRoot)) "Undefined" "MultiplyWithRoot" 0 0))
      (Variables|Default|SetOccupied? true)
      (bind _asbp_plant_base (Utilities|Casting|CastToBP_PlantBase _returnvalue_2))
      (bind _output_get (Variables|Default|SetCurrentPlant _asbp_plant_base))
      (Variables|/Game/Blueprints/IngameBlueprints/Plants/BP_PlantBase.BP_PlantBase_C|SetBP_FarmSpotRef _asbp_plant_base self)
      (Variables|Default|SetCurrentPlantID (.PlantID (Utilities|Struct|BreakST_PlantData _returnvalue)))
      (Variables|/Game/Blueprints/IngameBlueprints/Plants/BP_PlantBase.BP_PlantBase_C|SetCanBeBugTarget _output_get true))))

(fn Fertiled
  (Variables|Default|SetIsFertiled true)
  (Variables|Default|SetValueMultiplier 1.25))

(fn FertileReset
  (Variables|Default|SetIsFertiled false)
  (Variables|Default|SetValueMultiplier 1.0))

(fn ReplacePlant
  (Variables|Default|SetCurrentPlant (Variables|Default|GetUpdatedPlant)))

(fn ReturnInteractStatus
  (return (Variables|Default|GetIsInteractable)))

(fn ReturnSuccessfullyPlanted
  (return (Variables|Default|GetSuccessfullyPlanted?)))