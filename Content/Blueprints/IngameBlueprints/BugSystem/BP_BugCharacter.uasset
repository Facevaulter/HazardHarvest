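; Bug enemy character that hunts and damages plants, and can be killed by interaction, which notifies BP_DayNightManager.
; SearchTarget gathers living, non-mutated, targetable plants, then picks a random one by chance or else the nearest.
; AIMoveTo success starts a looping AttackPlant timer that drains PlantHealth and destroys the plant at zero.
; Target loss triggers a new search, and an empty target list tells the day/night manager to begin day.
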(event Custom|SearchTarget
  (bind _validtargets (Variables|Default|GetValidTargets))
  (Variables|Default|SetClosestDistance 999999.0)
  (Variables|Default|SetClosestPlant 0)
  (Utilities|Array|Clear (Variables|Default|GetValidTargets))
  (bind _outactors (Actor|GetAllActorsOfClass "/Game/Blueprints/IngameBlueprints/Plants/BP_PlantBase.BP_PlantBase_C"))
  (for _array_element _outactors
    (if (not (Variables|/Game/Blueprints/IngameBlueprints/Plants/BP_PlantBase.BP_PlantBase_C|GetMutated? _array_element))
      (if (Variables|/Game/Blueprints/IngameBlueprints/Plants/BP_PlantBase.BP_PlantBase_C|GetCanBeBugTarget _array_element)
        (if (> (Variables|/Game/Blueprints/IngameBlueprints/Plants/BP_PlantBase.BP_PlantBase_C|GetPlantHealth _array_element) 0.0)
          (Utilities|Array|Add (Variables|Default|GetValidTargets) _array_element)
          (Math|Integer|IncrementInt (Variables|Default|GetTotalTargets)
            (:%20%20
              (bind _output_get (Variables|Default|SetCurrentDistance (Transformation|GetDistanceTo _array_element self)))
              (if (< _output_get (Variables|Default|GetClosestDistance))
                (Variables|Default|SetClosestPlant _array_element)
                (Variables|Default|SetClosestDistance _output_get))))))))
  (if (> (Utilities|Array|Length (Variables|Default|GetValidTargets)) 0)
    (if (<= (Math|Float|Clamp(Float) (Math|Random|RandomFloat)) (Variables|Default|GetRandomSearchingBugChance))
      (Utilities|Array|Shuffle _validtargets)
      (bind _output_get_2 (Variables|Default|SetCurrentTarget (Utilities|Array|Get(acopy) _validtargets (Math|Random|RandomInteger (Variables|Default|GetTotalTargets)))))
      (Utilities|IsValid _output_get_2
        (:Is%20Valid
          (EventDispatchers|BindEventtoPlantDestroyed _output_get_2 (delegate Custom|TargetDestroyed))
          (AI|AIMoveTo self (Transformation|GetActorLocation _output_get_2) _output_get_2 5.0 false
            (:OnSuccess
              _))))
      (else
        (bind _output_get_3 (Variables|Default|SetCurrentTarget (Variables|Default|GetClosestPlant)))
        (Utilities|IsValid _output_get_3
          (:Is%20Valid
            (EventDispatchers|BindEventtoPlantDestroyed _output_get_3 (delegate Custom|TargetDestroyed))
            (AI|AIMoveTo self (Transformation|GetActorLocation _output_get_3) _output_get_3 5.0 false
              (:OnSuccess
                _))))))
    (Utilities|Time|SetTimerbyFunctionName 0 "AttackPlant" 0.5 true)))

(event Custom|CheckTargets
  (if (Utilities|Array|IsEmpty (Variables|Default|GetValidTargets))
    (bind _returnvalue (Actor|GetActorOfClass "/Game/Blueprints/IngameBlueprints/BP_DayNightManager.BP_DayNightManager_C"))
    (Default|BeginDay _returnvalue)))

(event Custom|TargetDestroyed
  (EventDispatchers|UnbindEventfromPlantDestroyed (Variables|Default|GetCurrentTarget) (delegate Custom|TargetDestroyed))
  (Variables|Default|SetCurrentTarget 0)
  (Utilities|Time|ClearTimerbyFunctionName 0 "AttackPlant")
  (CallFunction|SearchTarget)
  (CallFunction|CheckTargets))

(event EventInteract
  (params (Sender :type Actor%20Object%20Reference))
  (Utilities|IsValid self
    (:Is%20Valid
      (Default|BugKilled (Variables|Default|GetDayNightManagerRef))
      (Actor|DestroyActor))))

(event EventBeginPlay
  (bind _returnvalue (Actor|GetActorOfClass "/Game/Blueprints/IngameBlueprints/BP_DayNightManager.BP_DayNightManager_C"))
  (Variables|Default|SetDayNightManagerRef _returnvalue))

(fn ConstructionScript)

(fn AttackPlant
  (Utilities|IsValid (Variables|Default|GetCurrentTarget)
    (:Is%20Valid
      (if (Variables|/Game/Blueprints/IngameBlueprints/Plants/BP_PlantBase.BP_PlantBase_C|GetDestroyed? (Variables|Default|GetCurrentTarget))
        (CallFunction|SearchTarget)
        (else
          (Utilities|IsValid (Variables|Default|GetCurrentTarget)
            (:Is%20Valid
              (bind _output_get (Variables|/Game/Blueprints/IngameBlueprints/Plants/BP_PlantBase.BP_PlantBase_C|SetPlantHealth (Variables|Default|GetCurrentTarget) (- (Variables|/Game/Blueprints/IngameBlueprints/Plants/BP_PlantBase.BP_PlantBase_C|GetPlantHealth (Variables|Default|GetCurrentTarget)) (Variables|Default|GetDamage))))
              (if (<= _output_get 0.0)
                (Default|Destroy (Variables|Default|GetCurrentTarget))
                (Variables|Default|SetCurrentTarget 0)
                (Utilities|Time|ClearTimerbyFunctionName 0 "AttackPlant")
                (CallFunction|SearchTarget)
                (CallFunction|CheckTargets)))))))
    (:Is%20Not%20Valid
      (CallFunction|SearchTarget)
      (Utilities|Time|ClearTimerbyFunctionName 0 "AttackPlant")
      (return))))

(fn ReturnInteractStatus
  (return (Variables|Default|GetIsInteractable)))

(fn ReturnSuccessfullyPlanted
  (return false))