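; BP_Shop is an interactable shop actor that opens the buy menu when used.
; Interact proceeds only if the game mode's TaskshieldInteracted flag is set and the IsInteractable check passes.
; It then adds CAW_ShopBuy to the main widget stack, switches to UI-only input with a visible cursor, plays an opening sound, and hides the Ausrufezeichen (exclamation mark) actor once.
; Interaction functions set and report interactability, with planting success always false.
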(event EventBeginPlay)

(event Collision|EventActorBeginOverlap
  (params (OtherActor :type Actor%20Object%20Reference)))

(event EventTick
  (params (DeltaSeconds :type Float%20%28single-precision%29)))

(event EventInteract
  (params (Sender :type Actor%20Object%20Reference))
  (bind _asbp_game_mode (Utilities|Casting|CastToBP_GameMode (Game|GetGameMode)))
  (if (Variables|/Game/Blueprints/Core/BP_GameMode.BP_GameMode_C|GetTaskshieldInteracted _asbp_game_mode)
    (Variables|Default|GetIsInteractable
      (:then
        (Class|CommonActivatableWidgetContainerBase|AddWidget (Utilities|ReturnMainStack (Game|GetPlayerController 0)) "/Game/Blueprints/UI/CAW_ShopBuy.CAW_ShopBuy_C")
        (Variables|/Script/Engine.PlayerController|SetbShowMouseCursor (Game|GetPlayerController 0) true)
        (Input|SetInputModeUIOnly (Game|GetPlayerController 0) 0 "DoNotLock" false)
        (Audio|PlaySound2D "/Game/Assets/Sound/SFX/Shopping/SC_OpenShop.SC_OpenShop" 1.0 1.0 0.0 0 0)
        (Utilities|FlowControl|DoOnce false
          (:Completed
            (Rendering|SetActorHiddenInGame (Variables|Default|GetAusrufezeichen) true))))
      (:else))))

(event EventSetInteractStatus
  (params (IsInteractable :type Boolean))
  (Variables|Default|SetIsInteractable IsInteractable))

(fn ConstructionScript)

(fn ReturnInteractStatus
  (return (Variables|Default|GetIsInteractable)))

(fn ReturnSuccessfullyPlanted
  (return false))