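; Donation quest manager that sets plant donation quotas with a day deadline and ends the game when one is missed.
; Each goal grows in size, drawing random plants from PlantData, with a wider pool after early successes.
; DonatePlant tallies parallel arrays; completing a goal updates the donation station's sack and immediately rolls the next.
; Day/night dispatchers drive the countdown, resetting it at nightfall on success or showing the end-game screen.
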(event Custom|BeginDay
  (Math|Integer|DecrementInt (Variables|Default|GetDaysUntilDonationGoal)))

(event Custom|BeginNight
  (if (<= (Variables|Default|GetDaysUntilDonationGoal) 0)
    (Variables|Default|GetDonationGoalFullfilled
      (:then
        (Variables|Default|SetDaysUntilDonationGoal (Variables|Default|GetDonationInterval))
        (Variables|Default|SetDonationGoalFullfilled false)
        (Variables|Default|SetReadyForDelivery false)
        (bind _asbp_donation_station (Utilities|Casting|CastToBP_DonationStation (Variables|Default|GetDonationCart)))
        (Default|SackAus _asbp_donation_station))
      (:else
        (CallFunction|GameOverRoutine)))))

(event Custom|SetDonationGoal
  (Variables|Default|SetPlantAMountToDonate (+ (Variables|Default|GetPlantAMountToDonate) (Variables|Default|GetDonationAmountIncrease)))
  (Utilities|Array|Clear (Variables|Default|GetDonatedPlantsAmount))
  (Utilities|Array|Clear (Variables|Default|GetDonationGoalPlantID))
  (Utilities|Array|Clear (Variables|Default|GetDonationGoalAmount))
  (if (== (Variables|Default|GetDonationGoalsFullfilled) 0)
    (CallFunction|RandomDonationAmount 0 2 (Variables|Default|GetPlantAMountToDonate))
    (elif (== (Variables|Default|GetDonationGoalsFullfilled) 1)
      (CallFunction|RandomDonationAmount 0 4 (Variables|Default|GetPlantAMountToDonate))
      (else
        (CallFunction|RandomDonationAmount 0 6 (Variables|Default|GetPlantAMountToDonate))))))

(event EventBeginPlay
  (bind _daynightmanagerref (Variables|Default|GetDayNightManagerRef))
  (bind _outrownames (DataTable|GetDataTableRowNames (Variables|Default|GetPlantData)))
  (Variables|Default|SetPlantDataRowNames _outrownames)
  (EventDispatchers|BindEventtoBeginDayDispatcher _daynightmanagerref (EventDispatchers|CreateEvent :!event Custom|BeginDay))
  (EventDispatchers|BindEventtoBeginNightDispatcher _daynightmanagerref (EventDispatchers|CreateEvent :!event Custom|BeginNight))
  (bind _asbp_player (Utilities|Casting|CastToBP_Player (Game|GetPlayerCharacter 0)))
  (Variables|Default|SetPlayerRef _asbp_player)
  (Variables|Default|GetFirstDonationGoal
    (:then
      (Variables|Default|SetFirstDonationGoal false)
      (CallFunction|SetDonationGoal))
    (:else)))

(fn ConstructionScript)

(fn RandomDonationAmount
  (params (Min :type Integer) (Max :type Integer) (PlantAmount :type Integer))
  (for _index (range 1 PlantAmount)
    (bind _output_get (Variables|Default|SetTempPlantID (Utilities|Array|Get(acopy) (Variables|Default|GetPlantDataRowNames) (Math|Random|RandomIntegerinRange Min Max))))
    (if (Utilities|Array|ContainsItem (Variables|Default|GetDonationGoalPlantID) _output_get)
      (Math|Integer|IncrementInt (Utilities|Array|Get(acopy) (Variables|Default|GetDonationGoalAmount) (Utilities|Array|FindItem (Variables|Default|GetDonationGoalPlantID) _output_get)))
      (else
        (Utilities|Array|Add (Variables|Default|GetDonationGoalPlantID) _output_get)
        (Utilities|Array|Add (Variables|Default|GetDonationGoalAmount) 1)
        (Utilities|Array|Add (Variables|Default|GetDonatedPlantsAmount) 0)))))

(fn GameOverRoutine
  (Class|CommonActivatableWidgetContainerBase|AddWidget (Utilities|ReturnMainStack (Game|GetPlayerController 0)) "/Game/Blueprints/UI/CAW_EndGame.CAW_EndGame_C")
  (bind _asbp_hud (Utilities|Casting|CastToBP_HUD (HUD|GetHUD (Game|GetPlayerController 0))))
  (Default|RemoveInventory _asbp_hud))

(fn CheckDonationGoal
  (bind (_array_element _array_index) (Utilities|Array|ForEachLoopwithBreak (Variables|Default|GetDonationGoalAmount) :!label _label)
    (:LoopBody
      (if (== _array_element (Utilities|Array|Get(acopy) (Variables|Default|GetDonatedPlantsAmount) _array_index))
        (Variables|Default|SetDonationGoalFullfilled true)
        (bind _asbp_donation_station (Utilities|Casting|CastToBP_DonationStation (Variables|Default|GetDonationCart)))
        (Default|SackAn _asbp_donation_station)
        (else
          (Variables|Default|SetDonationGoalFullfilled false)
          (goto _label Break))))
    (:Completed
      (Variables|Default|GetDonationGoalFullfilled
        (:then
          (Variables|Default|SetReadyForDelivery true)
          (Math|Integer|IncrementInt (Variables|Default|GetDonationGoalsFullfilled)
            (:%20%20
              (CallFunction|SetDonationGoal))))
        (:else)))))

(fn DonatePlant
  (params (PlantID :type Name%20%28by%20ref%29))
  (bind _donationgoalplantid (Variables|Default|GetDonationGoalPlantID))
  (bind _donatedplantsamount (Variables|Default|GetDonatedPlantsAmount))
  (bind _returnvalue (Utilities|Array|FindItem _donationgoalplantid PlantID))
  (if (Utilities|Array|ContainsItem _donationgoalplantid PlantID)
    (if (Utilities|Array|IsValidIndex _donatedplantsamount _returnvalue)
      (Math|Integer|IncrementInt (Utilities|Array|Get(acopy) _donatedplantsamount _returnvalue)
        (:%20%20
          (CallFunction|CheckDonationGoal))))))