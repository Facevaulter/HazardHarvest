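; Interactable donation station that opens the donation UI once the game mode's TaskshieldInteracted flag is set.
; Interact hides its exclamation marker, then, if interactable, pushes CAW_Donation onto the main widget stack in UI-only input with cursor.
; The first successful use also reveals the shop's exclamation marker through a DoOnce.
; Separate events toggle the sack's visibility and set the interact status, which a getter returns.
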(event Custom|SackAn
  (Rendering|SetVisibility (Variables|Default|GetSack) true false))

(event Custom|SackAus
  (Rendering|SetVisibility (Variables|Default|GetSack) false false))

(event EventBeginPlay)

(event Collision|EventActorBeginOverlap
  (params (OtherActor :type Actor%20Object%20Reference)))

(event EventTick
  (params (DeltaSeconds :type Float%20%28single-precision%29)))

(event EventInteract
  (params (Sender :type Actor%20Object%20Reference))
  (bind _asbp_game_mode (Utilities|Casting|CastToBP_GameMode (Game|GetGameMode)))
  (if (Variables|/Game/Blueprints/Core/BP_GameMode.BP_GameMode_C|GetTaskshieldInteracted _asbp_game_mode)
    (Rendering|SetActorHiddenInGame (Variables|Default|GetAusrufezeichen) true)
    (Variables|Default|GetIsInteractable
      (:then
        (Class|CommonActivatableWidgetContainerBase|AddWidget (Utilities|ReturnMainStack (Game|GetPlayerController 0)) "/Game/Blueprints/UI/CAW_Donation.CAW_Donation_C")
        (Variables|/Script/Engine.PlayerController|SetbShowMouseCursor (Game|GetPlayerController 0) true)
        (Input|SetInputModeUIOnly (Game|GetPlayerController 0) 0 "DoNotLock" false)
        (Utilities|FlowControl|DoOnce false
          (:Completed
            (Rendering|SetActorHiddenInGame (Variables|Default|GetAusrufezeichenShop) false))))
      (:else))))

(event EventSetInteractStatus
  (params (IsInteractable :type Boolean))
  (Variables|Default|SetIsInteractable IsInteractable))

(fn ConstructionScript)

(fn ReturnInteractStatus
  (return (Variables|Default|GetIsInteractable)))

(fn ReturnSuccessfullyPlanted
  (return false))