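; BP_ExclamationMarkFirst is an exclamation mark actor that hovers up and down and can be shown or hidden.
; On BeginPlay it stores its start location and plays HoverTimeline, whose alpha drives a vertical offset around that point.
; Two custom events, ShowAusrufezeichen and HideAusrufezeichen, toggle the visibility of the Ausrufezeichen (German for exclamation mark) component.
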(event Custom|ShowAusrufezeichen
  (Rendering|SetVisibility (Variables|Default|GetAusrufezeichen) true false))

(event Custom|HideAusrufezeichen
  (Rendering|SetVisibility (Variables|Default|GetAusrufezeichen) false false))

(event EventBeginPlay
  (Variables|Default|SetStartLocation (Transformation|GetActorLocation))
  (bind _hoveralpha (Timeline|HoverTimeline Play)
    (:Update
      (Transformation|SetActorLocation (Math|Vector|MakeVector (.x (Variables|Default|GetStartLocation)) (.y (Variables|Default|GetStartLocation)) (+ (.z (Variables|Default|GetStartLocation)) (Math|Float|Lerp -2e+01 2e+01 _hoveralpha))) false false))))

(fn ConstructionScript)