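; BP_TaskShield is an interactable task board that opens the daily tasks screen.
; Interacting adds a new CAW_DailyTasks widget to the viewport and tells BP_GameMode to enable interaction with things other than the shield.
; A DoOnce then hides the board's exclamation mark actor (Ausrufezeichen) and shows the cart's marker on first use.
; Interaction availability comes from the IsInteractable flag, and the planted-success query always returns false.
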(event EventBeginPlay)

(event Collision|EventActorBeginOverlap
  (params (OtherActor :type Actor%20Object%20Reference)))

(event EventTick
  (params (DeltaSeconds :type Float%20%28single-precision%29)))

(event EventInteract
  (params (Sender :type Actor%20Object%20Reference))
  (bind _returnvalue (UserInterface|CreateWidget "/Game/Blueprints/UI/CAW_DailyTasks.CAW_DailyTasks_C"))
  (UserInterface|Viewport|AddtoViewport _returnvalue 30)
  (bind _asbp_game_mode (Utilities|Casting|CastToBP_GameMode (Game|GetGameMode)))
  (Default|EnableInteractOtherThanTaskshield _asbp_game_mode)
  (Utilities|FlowControl|DoOnce false
    (:Completed
      (Rendering|SetActorHiddenInGame (Variables|Default|GetAusrufezeichen) true)
      (Rendering|SetActorHiddenInGame (Variables|Default|GetAusrufezeichenCart) false))))

(fn ConstructionScript)

(fn ReturnInteractStatus
  (return (Variables|Default|GetIsInteractable)))

(fn ReturnSuccessfullyPlanted
  (return false))