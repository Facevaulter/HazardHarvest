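; BP_Player is the player Blueprint for a crop-planting game, handling camera-relative movement, interaction and the seed inventory.
; Movement is gated by CanMoveCheck, while interaction sphere-traces downward ahead of the player for BPI_Interact actors.
; Crop plots receive the interact message only when the current seed count is above zero; other interactables receive it directly.
; RemoveSeed decrements the count after successful planting and refreshes the inventory UI.
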(event Custom|RemoveSeed
  (params (SuccesfullyPlanted :type Boolean))
  (if SuccesfullyPlanted
    (bind _output (Utilities|InventoryCountCheck)
      (:MoreThanZero
        (Math|Integer|DecrementInt _output
          (:%20%20
            (Default|CheckInventory (Variables|Default|GetInventoryUI)))))
      (:ZeroSeeds
        (Default|CheckInventory (Variables|Default|GetInventoryUI))))
    (else
      (CallFunction|UnbindPlantedCheck))))

(event Custom|CheckInventory
  (Default|CheckInventory (Variables|Default|GetInventoryUI)))

(event Input|EnhancedActionEvents|EnhancedInputActionIA_Move
  (params (ActionValue :type Vector%202D%20Structure) (ElapsedSeconds :type Float%20%28double-precision%29) (TriggeredSeconds :type Float%20%28double-precision%29) (InputAction :type Input%20Action%20Object%20Reference :default "/Game/Input/IA_Move.IA_Move"))
  (bind _returnvalue (Game|GetPlayerCameraManager 0))
  (bind (_x _y) (Math|Vector2D|BreakVector2D ActionValue))
  (Utilities|CanMoveCheck
    (:true
      (Pawn|Input|AddMovementInput (Math|Transform|TransformDirection (Math|Transform|MakeTransform (Camera|GetCameraLocation _returnvalue) (Math|Rotator|MakeRotator 0.0 0.0 (.Yaw (Math|Rotator|BreakRotator (Camera|GetCameraRotation _returnvalue)))) "1.000000,1.000000,1.000000") (Math|Vector|MakeVector _y _x 0.0)) 1.0 false))))

(event Input|EnhancedActionEvents|EnhancedInputActionIA_Interact
  (params (ActionValue :type Boolean) (ElapsedSeconds :type Float%20%28double-precision%29) (TriggeredSeconds :type Float%20%28double-precision%29) (InputAction :type Input%20Action%20Object%20Reference :default "/Game/Input/IA_Interact.IA_Interact"))
  (:Started
    (Variables|Default|GetCanInteract
      (:then
        (bind _actortointereact (|InteractCheck))
        (bind _asbp_crop_plot_base (Utilities|Casting|CastToBP_CropPlotBase _actortointereact)
          (:then
            (Variables|Default|SetCropPlotToPlant _asbp_crop_plot_base)
            (Utilities|InventoryCountCheck
              (:MoreThanZero
                (Class|BPIInteract|Interact(Message) (Variables|Default|GetCropPlotToPlant) self)
                (Default|CallSuccessfullInteractDispatcher)
                (Variables|Default|SetCropPlotToPlant 0))))
          (:CastFailed
            (Class|BPIInteract|Interact(Message) _actortointereact self)
            (Default|CallSuccessfullInteractDispatcher))))
      (:else))))

(event EventBeginPlay
  (bind _asbp_game_instance (Utilities|Casting|CastToBP_GameInstance (Game|GetGameInstance)))
  (Variables|Default|SetSettingsSaveRef (Variables|/Game/Blueprints/Core/BP_GameInstance.BP_GameInstance_C|GetSettingsSaveRef _asbp_game_instance)))

(fn ConstructionScript)

(fn UnbindPlantedCheck
  (EventDispatchers|UnbindEventfromSuccesfullyPlanted (Variables|Default|GetCropPlotToPlant) (EventDispatchers|CreateEvent :!event Custom|RemoveSeed))
  (Variables|Default|SetCropPlotToPlant 0))